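; BP_TestActor is a test actor with a simple health system that destroys it when health runs out.
; On BeginPlay, Fn_SetHealth sets CurrentHealth to MaxHealth.
; AnyDamage subtracts incoming damage, clamps the result between zero and MaxHealth, and destroys the actor at zero.
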(event `self.ReceiveBeginPlay`
  ;[0.2253 1 0] Begin Play
  (`self.Fn_SetHealth`))

(event `self.ReceiveAnyDamage`
  (params (Damage :type "Float (single-precision)") (DamageType :type "DamageType Object Reference") (InstigatedBy :type "Controller Object Reference") (DamageCauser :type "Actor Object Reference"))
  ;[0.1487 1 0] Health System AI
  (set `self.currentHealth` (`KismetMathLibrary.FClamp` (- (`self.currentHealth`) Damage) 0.0 (`self.maxHealth`)))
  (if (<= (`self.currentHealth`) 0.0)
    (`self.K2_DestroyActor`)))

(fn `Fn_SetHealth`
  (set `self.currentHealth` (`self.maxHealth`)))

(fn `UserConstructionScript`)