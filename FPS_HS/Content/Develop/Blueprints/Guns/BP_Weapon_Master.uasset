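; Master weapon Blueprint that handles hitscan shooting, magazine ammo and reloading.
; FnShoot passes a game-time fire-rate gate (DelayBtwShots), then plays an AK47 sound, spends a round and line-traces from the barrel socket, with debug drawing, to apply damage.
; An empty magazine sets OutOfBullets.
; CE_GunReload, blocked while IsShooting and guarded by a DoOnce, locks shooting during a fixed delay, then refills the magazine.
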(event `self.ReceiveBeginPlay`
  ;[1 0.2854 0.9919] Begin Play
  (`self.Fn_InitValues`))

(event `CE_GunReload`
  ;[0.436 0.2545 1] Gun Reload Method
  (if (not (`self.isShooting`))
    (`/Engine/EditorBlueprintResources/StandardMacros.DoOnce` false :!label _label
      (:`Completed`
        (set `self.isReloading` true)
        (set `self.ableToShoot` false)
        (if (< (`self.currentMagSize`) (`self.maxMagSize`))
          (`GameplayStatics.PlaySoundAtLocation` "/Game/Sounds/Gun/Reload.Reload" (`self.GetSocketLocation` "None") (struct) 0.3 1.0 0.0 null null null null)
          (set `self.ableToReload` false)
          (`KismetSystemLibrary.Delay` 3.0)
          (set `self.currentMagSize` (`self.maxMagSize`))
          (set `self.ableToReload` true)
          (set `self.ableToShoot` true)
          (set `self.isReloading` false)
          (`KismetSystemLibrary.Delay` 0.2)
          (goto _label :!via `Reset`))))))

(fn `Fn_InitValues`
  ;[0.881 0.08891 1] Initial Values Default
  (`|ExecutionSequence`
    (:`then_0`
      (set `self.ableToReload` true))
    (:`then_1`
      (set `self.currentMagSize` (`self.maxMagSize`)))
    (:`then_2`
      (set `self.ableToShoot` true))))

(fn `Fn_Shoot`
  (bind (_returnvalue_location _returnvalue_rotation) (`KismetMathLibrary.BreakTransform` (`self.GetSocketTransform` "barrel")))
  (bind _returnvalue (`KismetSystemLibrary.GetGameTimeInSeconds`))
  (bind _xshot (`self.XShot`))
  ;[0.06679 0.1159 1] Shoot Method
  (if (`self.ableToShoot`)
    (if (not (`self.isReloading`))
      (set `self.ableToReload` false)
      (if (> (`self.currentMagSize`) 0.0)
        (set `self.isShooting` true)
        (if (== _xshot 0.0)
          (set `self.XShot` _returnvalue :!label _label)
          (`GameplayStatics.PlaySoundAtLocation` "/Game/Sounds/Gun/AK47_Single_Shot.AK47_Single_Shot" (`self.GetSocketLocation` "barrel") (struct) 1.0 1.0 0.0 null null null null)
          (set `self.currentMagSize` (- (`self.currentMagSize`) 1.0))
          (bind _outhit (`KismetSystemLibrary.LineTraceSingle` :`Start` _returnvalue_location :`End` (+ _returnvalue_location (* (`KismetMathLibrary.GetForwardVector` _returnvalue_rotation) (`self.Range`))) :`TraceChannel` "TraceTypeQuery1" :`bTraceComplex` true :`DrawDebugType` "ForDuration"))
          (`GameplayStatics.ApplyDamage` (`.HitActor` (`GameplayStatics.BreakHitResult` _outhit)) (`self.Damage`))
          (elif (not (> (+ _xshot (`self.timeBtwBullets`)) _returnvalue))
            (goto _label)))
        (else
          (set `self.outOfBullets` true))))))