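; BP_ExplosiveBarrel is a damageable barrel that explodes when its health runs out.
; It starts at MaxHealth, subtracts incoming damage with clamping, and triggers the explosion at zero.
; The explosion applies ExplosionDamage to every actor overlapping ExplosionRad, then destroys the barrel after a short delay.
; A HasExploded flag ensures it detonates only once.
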(event `self.ReceiveBeginPlay`
  (set `self.currentHealth` (`self.maxHealth`)))

(event `self.ReceiveAnyDamage`
  (params (Damage :type "Float (single-precision)") (DamageType :type "DamageType Object Reference") (InstigatedBy :type "Controller Object Reference") (DamageCauser :type "Actor Object Reference"))
  (set `self.currentHealth` (`KismetMathLibrary.FClamp` (- (`self.currentHealth`) Damage) 0.0 (`self.maxHealth`)))
  (if (<= (`self.currentHealth`) 0.0)
    (`self.CE_Explode`)))

(event `CE_Explode`
  (bind _explosionrad (`self.ExplosionRad`))
  (if (not (`self.bHasExploded`))
    (set `self.bHasExploded` true)
    (if (`KismetSystemLibrary.IsValid` _explosionrad)
      (for _array_element (`PrimitiveComponent.GetOverlappingActors` _explosionrad null)
        (`GameplayStatics.ApplyDamage` _array_element (`self.ExplosionDamage`)))
      (`KismetSystemLibrary.Delay` 0.2)
      (`self.K2_DestroyActor`))))

(fn `UserConstructionScript`)