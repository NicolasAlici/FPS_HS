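; BP_AI_Character is a simple enemy AI character that chases player 0 and damages actors it touches.
; On begin play it fills health to max and starts a move loop that re-issues AIMoveTo toward the player after a short delay.
; Incoming damage lowers clamped health and destroys the actor at zero.
; Attack collision overlaps apply fixed damage, throttled by a DoOnce that resets after a brief cooldown.
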(event `self.ReceiveBeginPlay`
  ;[0.1768 0.291 1] AI Begin Play
  (`|ExecutionSequence`
    (:`then_0`
      (`self.Fn_SetHealth`))
    (:`then_1`
      (`self.CE_AIMove`))))

(event `CE_AIMove`
  ;[0.03215 0.451 1] AI Movement
  (`|AIMoveTo` self (0.0 0.0 0.0) (`GameplayStatics.GetPlayerCharacter` 0)
    (:`then`
      (`KismetSystemLibrary.Delay` 0.5)
      (`self.CE_AIMove`))))

(event `self.ReceiveAnyDamage`
  (params (Damage :type "Float (single-precision)") (DamageType :type "DamageType Object Reference") (InstigatedBy :type "Controller Object Reference") (DamageCauser :type "Actor Object Reference"))
  ;[0.2111 1 0.07339] AI Health System
  (set `self.currentHealth` (`KismetMathLibrary.FClamp` (- (`self.currentHealth`) Damage) 0.0 (`self.maxHealth`)))
  (if (<= (`self.currentHealth`) 0.0)
    (`self.K2_DestroyActor`)))

(event `self.AttackCollision.OnComponentBeginOverlap`
  (params (OverlappedComponent :type "PrimitiveComponent Object Reference") (OtherActor :type "Actor Object Reference") (OtherComp :type "PrimitiveComponent Object Reference") (OtherBodyIndex :type Integer) (bFromSweep :type Boolean) (SweepResult :type "HitResult Structure (by ref)"))
  ;[0.1752 0.617 1] AI Attack
  (`/Engine/EditorBlueprintResources/StandardMacros.DoOnce` false :!label _label
    (:`Completed`
      (`GameplayStatics.ApplyDamage` OtherActor 10.0)
      (`KismetSystemLibrary.Delay` 0.2)
      (goto _label :!via `Reset`))))

(fn `Fn_SetHealth`
  (set `self.currentHealth` (`self.maxHealth`)))

(fn `UserConstructionScript`)